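; BP_4ColorSwitch is an interactable switch that checks a player's UI answer against a correct answer.
; Its collision box shows prompt text and enables input on overlap, letting F toggle the switch widget and mouse cursor.
; The widget, created at BeginPlay, reports answers through a dispatcher, and the switch calls OnAnswerRight or OnAnswerWrong.
; Leaving the box hides the prompt, disables input and closes the widget.
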(event OnComponentBeginOverlap(boxCollision)
  (params (OverlappedComponent :type Primitive%20Component%20Object%20Reference) (OtherActor :type Actor%20Object%20Reference) (OtherComp :type Primitive%20Component%20Object%20Reference) (OtherBodyIndex :type Integer) (bFromSweep :type Boolean) (SweepResult :type Hit%20Result%20Structure%20%28by%20ref%29))
  (Rendering|SetVisibility (Variables|Default|GetText) true false)
  (Input|EnableInput (Game|GetPlayerController 0)))

(event OnComponentEndOverlap(boxCollision)
  (params (OverlappedComponent :type Primitive%20Component%20Object%20Reference) (OtherActor :type Actor%20Object%20Reference) (OtherComp :type Primitive%20Component%20Object%20Reference) (OtherBodyIndex :type Integer))
  (Rendering|SetVisibility (Variables|Default|GetText) false false)
  (Input|DisableInput (Game|GetPlayerController 0))
  (Widget|RemovefromParent (Variables|Default|GetswitchUI))
  (Variables|Default|SetisShowUI false)
  (Variables|/Script/Engine.PlayerController|SetbShowMouseCursor (Game|GetPlayerController 0) false))

(event Custom|OnUserAnswer
  (params (userinput :type Integer))
  (if (== userinput (Variables|Default|GetCorrectAnswer))
    (Default|CallOnAnswerRight userinput)
    (else
      (Default|CallOnAnswerWrong userinput))))

(event EventBeginPlay
  (Utilities|FlowControl|Sequence
    (:then_1
      (bind _returnvalue (UserInterface|CreateWidget "/Game/asset/BP_4ColorSwitch/BP_Swtich_UI.BP_Swtich_UI_C"))
      (Variables|Default|SetswitchUI _returnvalue))
    (:then_2
      (EventDispatchers|BindEventtoOnUserAnswer (Variables|Default|GetswitchUI) (delegate Custom|OnUserAnswer)))))

(event EventTick
  (params (DeltaSeconds :type Float%20%28single-precision%29)))

(event Input|KeyboardEvents|F
  (params (Key :type Key%20Structure :default "None"))
  (bind _returnvalue (Game|GetPlayerController 0))
  (bind _switchui (Variables|Default|GetswitchUI))
  (:Pressed
    (if (Variables|Default|GetisShowUI)
      (Widget|RemovefromParent _switchui)
      (Variables|Default|SetisShowUI false)
      (Variables|/Script/Engine.PlayerController|SetbShowMouseCursor _returnvalue false)
      (else
        (UserInterface|Viewport|AddtoViewport _switchui 0)
        (Variables|Default|SetisShowUI true)
        (Variables|Default|SetisShowUI true)
        (Variables|/Script/Engine.PlayerController|SetbShowMouseCursor _returnvalue true)))))

(fn ConstructionScript)